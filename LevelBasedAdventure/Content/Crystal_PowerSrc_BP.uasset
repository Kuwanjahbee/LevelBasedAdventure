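; Crystal power source Blueprint that lights up four point lights when an actor enters a trigger volume.
; The trigger volume's begin-overlap event checks that self is valid, then sets one shared high intensity on all four PointLightComponents.
; The overlapping actor is not filtered, and nothing turns the lights back down.
; BeginPlay, Tick, the actor's own overlap event and the construction script are empty.
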(event OnActorBeginOverlap(TriggerVolume)
  (params (OverlappedActor :type Actor%20Object%20Reference) (OtherActor :type Actor%20Object%20Reference))
  (Utilities|IsValid self
    (:Is%20Valid
      (Rendering|Components|Light|SetIntensity (Variables|/Script/Engine.PointLight|GetPointLightComponent (Variables|Default|GetPointLight)) 1e+04))))

(event EventBeginPlay)

(event Collision|EventActorBeginOverlap
  (params (OtherActor :type Actor%20Object%20Reference)))

(event EventTick
  (params (DeltaSeconds :type Float%20%28single-precision%29)))

(fn ConstructionScript)